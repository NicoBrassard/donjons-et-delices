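; BP_Cooking_Station is a cooking station that detects when the player pawn steps onto or off it.
; Begin and end overlaps on its StepOnCollision component filter for player 0's pawn and print the same debug line.
; Each then casts that pawn's controller to BP_TopDownPC_Combat_01 and calls EventCookingStart or EventCookingEnd, leaving the cooking logic to the controller.
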(event `self.StepOnCollision.OnComponentBeginOverlap`
  (params (OverlappedComponent :type "PrimitiveComponent Object Reference") (OtherActor :type "Actor Object Reference") (OtherComp :type "PrimitiveComponent Object Reference") (OtherBodyIndex :type Integer) (bFromSweep :type Boolean) (SweepResult :type "HitResult Structure (by ref)"))
  (bind _returnvalue (`GameplayStatics.GetPlayerPawn` 0))
  (if (== OtherActor _returnvalue)
    (`KismetSystemLibrary.PrintString` "Do you smell what the rock is cooking?")
    (bind _asbp_top_down_pc_combat_01 (cast `/Game/ThirdPerson/Blueprints/BP_TopDownPC_Combat_01` (`Pawn.GetController` _returnvalue)))
    (`/Game/ThirdPerson/Blueprints/BP_TopDownPC_Combat_01.Event CookingStart` _asbp_top_down_pc_combat_01)))

(event `self.StepOnCollision.OnComponentEndOverlap`
  (params (OverlappedComponent :type "PrimitiveComponent Object Reference") (OtherActor :type "Actor Object Reference") (OtherComp :type "PrimitiveComponent Object Reference") (OtherBodyIndex :type Integer))
  (bind _returnvalue (`GameplayStatics.GetPlayerPawn` 0))
  (if (== OtherActor _returnvalue)
    (`KismetSystemLibrary.PrintString` "Do you smell what the rock is cooking?")
    (bind _asbp_top_down_pc_combat_01 (cast `/Game/ThirdPerson/Blueprints/BP_TopDownPC_Combat_01` (`Pawn.GetController` _returnvalue)))
    (`/Game/ThirdPerson/Blueprints/BP_TopDownPC_Combat_01.Event CookingEnd` _asbp_top_down_pc_combat_01)))

(fn `UserConstructionScript`)