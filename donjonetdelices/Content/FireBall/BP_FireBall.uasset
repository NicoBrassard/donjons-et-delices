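; BP_FireBall is a fireball projectile that destroys itself on hit or after ten seconds.
; Its sphere ignores the instigator while moving, so it does not collide with whoever fired it.
; Hitting the combat player character triggers HitReact with the BP_Boss1 instigator's AttackDamage stat, unless the player controller's Imune flag is set.
; Hits spawn an explosion, except against an immune player, whom the sphere is set to ignore before destruction.
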(event `self.ReceiveBeginPlay`
  (`PrimitiveComponent.IgnoreActorWhenMoving` (`self.Sphere`) (`self.GetInstigator`) true)
  (`KismetSystemLibrary.Delay` 10.0)
  (`/Engine/EditorBlueprintResources/StandardMacros.IsValid` self
    (:`Is Valid`
      (`self.K2_DestroyActor`))))

(event `self.ReceiveHit`
  (params (MyComp :type "PrimitiveComponent Object Reference") (Other :type "Actor Object Reference") (OtherComp :type "PrimitiveComponent Object Reference") (bSelfMoved :type Boolean) (HitLocation :type "Vector Structure") (HitNormal :type "Vector Structure") (NormalImpulse :type "Vector Structure") (Hit :type "HitResult Structure (by ref)"))
  (bind _asbp_third_person_character_combat_01 (cast `/Game/ThirdPerson/Blueprints/BP_ThirdPersonCharacter_Combat_01` Other)
    (:`then`
      (bind _asbp_top_down_pc_combat_01 (cast `/Game/ThirdPerson/Blueprints/BP_TopDownPC_Combat_01` (`GameplayStatics.GetPlayerController` 0))
        (:`then`
          (if (`/Game/ThirdPerson/Blueprints/BP_TopDownPC_Combat_01.Imune` _asbp_top_down_pc_combat_01)
            (`PrimitiveComponent.IgnoreActorWhenMoving` (`self.Sphere`) (`GameplayStatics.GetPlayerCharacter` 0) true)
            (else
              (bind _asbp_boss_1 (cast `/Game/ThirdPerson/Blueprints/BP_Boss1` (`self.GetInstigator`))
                (:`then`
                  (`/Game/ThirdPerson/Blueprints/BP_ThirdPersonCharacter_Combat_01.HitReact` _asbp_third_person_character_combat_01 (`/Game/ThirdPerson/Blueprints/MonsterStatsComponent.GetStat` (`/Game/ThirdPerson/Blueprints/BP_Boss1.MonsterStatsComponent` _asbp_boss_1) "AttackDamage")))
                (:`CastFailed`
                  _))
              (`GameplayStatics.SpawnEmitterAtLocation` "/Game/StarterContent/Particles/P_Explosion.P_Explosion" HitLocation :!label _label))))
        (:`CastFailed`
          (goto _label))))
    (:`CastFailed`
      (goto _label)))
  (`self.K2_DestroyActor`))

(fn `UserConstructionScript`)